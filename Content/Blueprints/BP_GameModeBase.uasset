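; Game mode Blueprint that runs a countdown of about three minutes and quits the game when it expires.
; BeginPlay seeds the Minutes and Seconds variables.
; Tick passes through a one-second Delay, throttling it to roughly one decrement per second, rolls Seconds over into Minutes, and calls QuitGame when both reach zero.
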(event `self.ReceiveBeginPlay`
  (set `self.Minutes` 2)
  (set `self.Seconds` 59))

(event `self.ReceiveTick`
  (params (DeltaSeconds :type "Float (single-precision)"))
  (`KismetSystemLibrary.Delay` 1.0)
  (set `self.Seconds` (- (`self.Seconds`) 1))
  (if (< (`self.Seconds`) 0)
    (set `self.Minutes` (- (`self.Minutes`) 1))
    (set `self.Seconds` 59))
  (if (== (`self.Seconds`) 0)
    (if (== (`self.Minutes`) 0)
      (`KismetSystemLibrary.QuitGame` null "Quit"))))

(fn `UserConstructionScript`)